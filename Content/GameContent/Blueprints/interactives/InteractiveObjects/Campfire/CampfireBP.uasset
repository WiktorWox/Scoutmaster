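; Campfire interactive object that the player can light and then use as a save point.
; On BeginPlay it hands itself to its PaperZD animation instance (CampfireAnimBP).
; Interacting while unlit flags the player as lighting and passes it the campfire reference; interacting once Fires is set writes a fresh, unpopulated SaveGame object to slot "1" and prints a Polish "game saved" message.
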(event EventBeginPlay
  (bind _ascampfire_anim_bp (Utilities|Casting|CastToCampfireAnimBP (Variables|/Script/PaperZD.PaperZDAnimationComponent|GetAnimInstance (Variables|Default|GetPaperZDAnimation))))
  (Variables|/Game/GameContent/Blueprints/interactives/InteractiveObjects/Campfire/CampfireAnimBP.CampfireAnimBP_C|SetCampfireRef _ascampfire_anim_bp self)
  (|CallParentFunction))

(event Collision|EventActorBeginOverlap
  (params (OtherActor :type Actor%20Object%20Reference)))

(event EventTick
  (params (DeltaSeconds :type Float%20%28single-precision%29)))

(fn ConstructionScript
  (|CallParentFunction))

(fn OnInteract
  (params (PlayerRef :type Player%20BP%20Object%20Reference))
  (bind _fires (Variables|Default|GetFires))
  (if (and (not (Variables|Default|GetFiresUp)) (not _fires))
    (Variables|/Game/GameContent/Blueprints/player/PlayerBP.PlayerBP_C|SetIsLightning PlayerRef true)
    (Variables|/Game/GameContent/Blueprints/player/PlayerBP.PlayerBP_C|SetCampFireRef PlayerRef self)
    (|CallParentFunction PlayerRef)
    (elif _fires
      (bind _returnvalue (SaveGame|CreateSaveGameObject "/Game/GameContent/Blueprints/SaveGame.SaveGame_C"))
      (bind _output_get (Variables|Default|SetSaveGameInstance _returnvalue))
      (bind _returnvalue_2 (SaveGame|SaveGametoSlot _output_get "1" (Variables|/Game/GameContent/Blueprints/SaveGame.SaveGame_C|GetUserIndex _output_get)))
      (if _returnvalue_2
        (Development|PrintString "Gra Zapisana!")))))