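; DoorBP is an interactive door object that opens a UI when a player interacts with it.
; OnInteract sets the player's IsUIOpened flag, adds the player's existing ZoomUI widget to the viewport, then calls the parent implementation.
; The Blueprint has no door movement logic of its own, and its event graph holds only disabled default events.
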(event EventBeginPlay
  (|CallParentFunction) ; This node is disabled and will not be called.\nDrag off pins to build functionality.
)

(event Collision|EventActorBeginOverlap
  (params (OtherActor :type Actor%20Object%20Reference))
  (|CallParentFunction OtherActor) ; This node is disabled and will not be called.\nDrag off pins to build functionality.
)

(event EventTick
  (params (DeltaSeconds :type Float%20%28single-precision%29))
  (|CallParentFunction DeltaSeconds) ; This node is disabled and will not be called.\nDrag off pins to build functionality.
)

(fn ConstructionScript
  (|CallParentFunction))

(fn OnInteract
  (params (PlayerRef :type Player%20BP%20Object%20Reference))
  (Variables|/Game/GameContent/Blueprints/player/PlayerBP.PlayerBP_C|SetIsUIOpened PlayerRef true)
  (UserInterface|Viewport|AddtoViewport (Variables|/Game/GameContent/Blueprints/player/PlayerBP.PlayerBP_C|GetZoomUI PlayerRef) 0)
  (|CallParentFunction PlayerRef))