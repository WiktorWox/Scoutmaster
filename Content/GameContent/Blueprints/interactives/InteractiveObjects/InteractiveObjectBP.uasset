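; InteractiveObjectBP is a Blueprint base for interactive objects that show a marker and pass a tip to the player.
; Interact sets a flipbook on the Mark component, copies its tip text and sprite onto the player reference, then calls the parent.
; StopInteract clears the mark and tip before calling the parent.
; OnInteract and EndInteract are empty, and the event graph holds only disabled default events.
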(event EventBeginPlay
  (|CallParentFunction) ; This node is disabled and will not be called.\nDrag off pins to build functionality.
)

(event Collision|EventActorBeginOverlap
  (params (OtherActor :type Actor%20Object%20Reference)))

(event EventTick
  (params (DeltaSeconds :type Float%20%28single-precision%29)))

(fn ConstructionScript
  (|CallParentFunction))

(fn ShowMark
  (Sprite|SetFlipbook (Variables|Default|GetMark) "/Game/GameContent/GameAssets/environment/InteractiveObjects/mark_flipbook.mark_flipbook"))

(fn HideMark
  (Sprite|SetFlipbook (Variables|Default|GetMark)))

(fn Interact
  (params (PlayerRef :type Player%20BP%20Object%20Reference))
  (CallFunction|ShowMark)
  (Variables|/Game/GameContent/Blueprints/player/PlayerBP.PlayerBP_C|SetTipText PlayerRef (Variables|Default|GetTipText))
  (Variables|/Game/GameContent/Blueprints/player/PlayerBP.PlayerBP_C|SetTipSprite PlayerRef (Variables|Default|GetTipSprite))
  (|CallParentFunction PlayerRef))

(fn StopInteract
  (params (PlayerRef :type Player%20BP%20Object%20Reference))
  (CallFunction|HideMark)
  (Variables|/Game/GameContent/Blueprints/player/PlayerBP.PlayerBP_C|SetTipText PlayerRef "")
  (Variables|/Game/GameContent/Blueprints/player/PlayerBP.PlayerBP_C|SetTipSprite PlayerRef 0)
  (|CallParentFunction PlayerRef))

(fn OnInteract
  (params (PlayerRef :type Player%20BP%20Object%20Reference)))

(fn EndInteract
  (params (PlayerRef :type Player%20BP%20Object%20Reference)))