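; Interactive object Blueprint that lets the player sit down, built on a parent interactive class that it calls through on each event.
; BeginPlay sets a Polish "Usiadz" (sit) prompt and E-key sprite.
; OnInteract flags the player as sitting, snaps the control rotation to a fixed yaw, hides the mark and switches the prompt to "Wstan" (stand up).
; EndInteract restores the mark and prompt, leaving any further reset to the parent.
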(event EventBeginPlay
  (Variables|Default|SetTipText "Usiadz")
  (Variables|Default|SetTipSprite "/Game/GameContent/GameAssets/sprites/Alert/e_Sprite.e_Sprite")
  (|CallParentFunction))

(event Collision|EventActorBeginOverlap
  (params (OtherActor :type Actor%20Object%20Reference))
  (|CallParentFunction OtherActor) ; This node is disabled and will not be called.\nDrag off pins to build functionality.
)

(event EventTick
  (params (DeltaSeconds :type Float%20%28single-precision%29))
  (|CallParentFunction DeltaSeconds) ; This node is disabled and will not be called.\nDrag off pins to build functionality.
)

(fn ConstructionScript
  (|CallParentFunction))

(fn OnInteract
  (params (PlayerRef :type Player%20BP%20Object%20Reference))
  (Variables|/Game/GameContent/Blueprints/player/PlayerBP.PlayerBP_C|SetIsSittingDown PlayerRef true)
  (Pawn|SetControlRotation (Pawn|GetController PlayerRef) (Math|Rotator|MakeRotator 0.0 0.0 1.8e+02))
  (CallFunction|HideMark)
  (Variables|/Game/GameContent/Blueprints/player/PlayerBP.PlayerBP_C|SetTipText PlayerRef "Wstan")
  (|CallParentFunction PlayerRef))

(fn EndInteract
  (params (PlayerRef :type Player%20BP%20Object%20Reference))
  (CallFunction|ShowMark)
  (Variables|/Game/GameContent/Blueprints/player/PlayerBP.PlayerBP_C|SetTipText PlayerRef "Usiadz")
  (|CallParentFunction PlayerRef))