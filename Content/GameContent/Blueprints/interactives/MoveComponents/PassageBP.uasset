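; PassageBP is an interactive passage that gates the player's ability to walk while interacting with it.
; Interact enables the player's CanWalk flag unless IsWalkingUp is set, and StopInteract clears it.
; It stores two layer references through SetLayers and exposes them through GetLayers.
; WalkUp and WalkDown are empty stubs, and the event graph holds no active logic.
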(event EventBeginPlay
  (|CallParentFunction) ; This node is disabled and will not be called.\nDrag off pins to build functionality.
)

(event Collision|EventActorBeginOverlap
  (params (OtherActor :type Actor%20Object%20Reference)))

(event EventTick
  (params (DeltaSeconds :type Float%20%28single-precision%29)))

(fn ConstructionScript
  (|CallParentFunction))

(fn Interact
  (params (PlayerRef :type Player%20BP%20Object%20Reference))
  (if (not (Variables|/Game/GameContent/Blueprints/player/PlayerBP.PlayerBP_C|GetIsWalkingUp PlayerRef))
    (Variables|/Game/GameContent/Blueprints/player/PlayerBP.PlayerBP_C|SetCanWalk PlayerRef true)))

(fn StopInteract
  (params (PlayerRef :type Player%20BP%20Object%20Reference))
  (Variables|/Game/GameContent/Blueprints/player/PlayerBP.PlayerBP_C|SetCanWalk PlayerRef false))

(fn SetLayers
  (params (Layer0 :type Layer%20BP%20Object%20Reference) (Layer1 :type Layer%20BP%20Object%20Reference))
  (Variables|Default|SetLayer0Ref Layer0)
  (Variables|Default|SetLayer1Ref Layer1))

(fn GetLayers
  (return (Variables|Default|GetLayer0Ref) (Variables|Default|GetLayer1Ref)))

(fn WalkUp)

(fn WalkDown)