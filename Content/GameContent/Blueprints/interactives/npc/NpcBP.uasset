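; Base interactable NPC Blueprint whose Alert sprite swaps to an E prompt on Interact and back on StopInteract.
; Tick drives an idle timer with a random AFK roll, but it passes zero delta and never sets the AFK flag true.
; Interacted only checks the player for a speaker component.
; UpdateControlRotation is empty, leaving its left/right facing logic from X velocity disconnected.
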(event Custom|UpdateControlRotation)

(event Custom|IdleTimerEvent
  (params (Delta%20Seconds :type Float%20%28double-precision%29))
  (if (not (Variables|Default|GetIsNpcAfk))
    (bind _output_get (Variables|Default|SetIdleTimer (+ Delta%20Seconds (Variables|Default|GetIdleTimer))))
    (if (> _output_get 1e+01)
      (if (== (Math|Float|Round (* (Math|Random|RandomFloat) 1.0)) 0)
        (Variables|Default|SetIsNpcAfk false)
        (else
          (Variables|Default|SetIdleTimer 0.0))))))

(event Custom|Interacted
  (params (PlayerRef :type Player%20BP%20Object%20Reference))
  (Utilities|IsValid (Actor|GetComponentbyClass PlayerRef "/DialogueTree/Blueprints/SpeakerComponents/BPC_SpeakerComponent.BPC_SpeakerComponent_C")))

(event EventBeginPlay
  (Variables|Default|SetIsAlert true)
  (|CallParentFunction))

(event EventTick
  (params (DeltaSeconds :type Float%20%28single-precision%29))
  (CallFunction|IdleTimerEvent 0.0)
  (CallFunction|UpdateControlRotation))

(fn ConstructionScript
  (|CallParentFunction))

(fn Interact
  (params (PlayerRef :type Player%20BP%20Object%20Reference))
  (Rendering|Components|Sprite|SetSprite (Variables|Default|GetAlert) "/Game/GameContent/GameAssets/sprites/Alert/e_Sprite.e_Sprite"))

(fn StopInteract
  (params (PlayerRef :type Player%20BP%20Object%20Reference))
  (Rendering|Components|Sprite|SetSprite (Variables|Default|GetAlert) "/Game/GameContent/GameAssets/sprites/Alert/alert_Sprite.alert_Sprite"))