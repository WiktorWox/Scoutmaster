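; An NPC character Blueprint that faces its direction of travel, talks when interacted with and can be sent to a target.
; Each tick it snaps control rotation to one of two opposite yaws from the sign of X velocity.
; While flagged AFK, a timer periodically randomly either clears the flag or restarts the wait.
; Interaction starts its own speaker component's dialogue with the player's, and MoveTo uses AI Move To toward an actor.
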(event Custom|UpdateControlRotation
  ;[1 1 1] PlayerRotation
  (Utilities|IsValid (Pawn|GetController)
    (:Is%20Valid
      (Math|Float|CompareFloat (.X (Math|Vector|BreakVector (Variables|/Script/Engine.MovementComponent|GetVelocity (Variables|Character|GetCharacterMovement)))) 0.0
        (:>
          (Pawn|SetControlRotation (Pawn|GetController) (Math|Rotator|MakeRotator 0.0 0.0 0.0)))
        (:<
          (Pawn|SetControlRotation (Pawn|GetController) (Math|Rotator|MakeRotator 0.0 0.0 1.8e+02)))))))

(event Custom|IdleTimerEvent
  (params (Delta%20Seconds :type Float%20%28double-precision%29))
  (if (Variables|Default|GetIsNpcAfk)
    (bind _output_get (Variables|Default|SetIdleTimer (+ Delta%20Seconds (Variables|Default|GetIdleTimer))))
    (if (> _output_get 1e+01)
      (if (== (Math|Float|Round (* (Math|Random|RandomFloat) 1.0)) 0)
        (Variables|Default|SetIsNpcAfk false)
        (else
          (Variables|Default|SetIdleTimer 0.0))))))

(event Custom|Interacted
  (params (PlayerRef :type Player%20BP%20Object%20Reference))
  (bind _returnvalue (Actor|GetComponentbyClass PlayerRef "/DialogueTree/Blueprints/SpeakerComponents/BPC_SpeakerComponent.BPC_SpeakerComponent_C"))
  (Utilities|IsValid _returnvalue
    (:Is%20Valid
      (Class|DialogueSpeakerComponent|StartOwnedDialogue (Variables|Default|GetBPC_SpeakerComponent) (Utilities|Array|MakeArray _returnvalue)))))

(event Custom|MoveTo
  (params (Destination :type Vector))
  (AI|AIMoveTo self "0, 0, 0" (Variables|Default|GetDestination) 5.0 false))

(event EventTick
  (params (DeltaSeconds :type Float%20%28single-precision%29))
  (CallFunction|IdleTimerEvent DeltaSeconds)
  (CallFunction|UpdateControlRotation))

(fn ConstructionScript)