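; Drag-and-drop operation for Prowe tiles in the backpack's badge UI, handling what happens when a drag is cancelled.
; If the drag has a valid index, it writes the carried tile content back into that slot of the Prowe component and refreshes the backpack widget's grid.
; Otherwise, it makes the referenced tile visible again.
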(event EventDragCancelled
  (params (PointerEvent :type Pointer%20Event%20Structure%20%28by%20ref%29))
  (if (!= (Variables|Default|GetIndex) -1)
    (Default|SetTile (Variables|Default|GetProweCompRef) (Variables|Default|GetTileContent) (Variables|Default|GetIndex))
    (Default|RefreshGrid (Variables|Default|GetBackPackWidgetRef))
    (else
      (Variables|/Script/UMG.Widget|SetVisibility (Variables|Default|GetTileRef) "Visible"))))