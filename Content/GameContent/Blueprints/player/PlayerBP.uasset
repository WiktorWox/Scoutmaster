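; Player pawn for a layered 2D side-scroller using PaperZD, handling movement, interaction and UI.
; Enhanced Input drives walking, with the spring arm following within the current layer's width and control rotation flipping by velocity.
; Overlapped PassageBP actors start stair transitions between layers; interaction reaches NPC dialogue, interactive objects or getting up from sitting.
; CanDoSth gates most actions on state flags, alongside inventory toggling and an AFK idle timer.
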(event Custom|UpdateControlRotation
  ;[1 1 1] PlayerRotation
  (Utilities|IsValid (Pawn|GetController)
    (:Is%20Valid
      (Math|Float|CompareFloat (.X (Math|Vector|BreakVector (Variables|/Script/Engine.MovementComponent|GetVelocity (Variables|Character|GetCharacterMovement)))) 0.0
        (:>
          (Pawn|SetControlRotation (Pawn|GetController) (Math|Rotator|MakeRotator 0.0 0.0 0.0)))
        (:<
          (Pawn|SetControlRotation (Pawn|GetController) (Math|Rotator|MakeRotator 0.0 0.0 1.8e+02)))))))

(event Custom|IdleTimerEvent
  (params (Delta%20Seconds :type Float%20%28double-precision%29))
  (if (not (Variables|Default|GetIsPlayerAfk))
    (bind _output_get (Variables|Default|SetIdleTimer (+ Delta%20Seconds (Variables|Default|GetIdleTimer))))
    (if (> _output_get 1e+01)
      (if (== (Math|Float|Round (* (Math|Random|RandomFloat) 1.0)) 0)
        (Variables|Default|SetIsPlayerAfk false)
        (else
          (Variables|Default|SetIdleTimer 0.0))))))

(event Custom|ChangeFallingSpeed
  (params (Delta%20Seconds :type Float%20%28double-precision%29))
  (if (AI|Components|NavMovement|IsFalling (Variables|Character|GetCharacterMovement))
    (if (<= (Components|Movement|GetGravityZ (Variables|Character|GetCharacterMovement)) 0.0)
      (Character|LaunchCharacter (Math|Vector|MakeVector 0.0 0.0 (* Delta%20Seconds 1e+03)) false false))))

(event Input|EnhancedActionEvents|EnhancedInputActionIA_anykey
  (params (ActionValue :type Float%20%28double-precision%29) (ElapsedSeconds :type Float%20%28double-precision%29) (TriggeredSeconds :type Float%20%28double-precision%29) (InputAction :type Input%20Action%20Object%20Reference :default "/Game/GameContent/Blueprints/IA_anykey.IA_anykey"))
  (Variables|Default|SetIdleTimer 0.0)
  (Variables|Default|SetIsPlayerAfk false))

(event Input|EnhancedActionEvents|EnhancedInputActionIA_inventory_menu
  (params (ActionValue :type Float%20%28double-precision%29) (ElapsedSeconds :type Float%20%28double-precision%29) (TriggeredSeconds :type Float%20%28double-precision%29) (InputAction :type Input%20Action%20Object%20Reference :default "/Game/GameContent/Blueprints/IA_inventory_menu.IA_inventory_menu"))
  ;[1 1 1] Controls
  (if (not (Variables|Default|GetIsUIOpened))
    (Variables|Default|SetIsUIOpened true)
    (UserInterface|Viewport|AddtoViewport (Variables|Default|GetInventoryUI) 0)
    (else
      (Variables|Default|SetIsUIOpened false)
      (Widget|RemovefromParent (Variables|Default|GetInventoryUI))
      (Input|SetInputModeGameOnly (Game|GetPlayerController 0) false))))

(event Input|EnhancedActionEvents|EnhancedInputActionIA_walk_up
  (params (ActionValue :type Float%20%28double-precision%29) (ElapsedSeconds :type Float%20%28double-precision%29) (TriggeredSeconds :type Float%20%28double-precision%29) (InputAction :type Input%20Action%20Object%20Reference :default "/Game/GameContent/Blueprints/IA_walk_up.IA_walk_up"))
  ;[1 1 1] Controls
  (bind _candosth (CallFunction|CanDoSth))
  (if _candosth
    (bind _array_element (Utilities|Array|ForEachLoopwithBreak (Collision|GetOverlappingActors "/Game/GameContent/Blueprints/interactives/InteractiveBaseBP.InteractiveBaseBP_C" :!class /Script/Engine.Actor) :!label _label)
      (:LoopBody
        (if (Actor|ActorHasTag _array_element "MoveComponent")
          (bind _aspassage_bp (Utilities|Casting|CastToPassageBP _array_element))
          (bind _layer0ref (Default|GetLayers _aspassage_bp))
          (bind _currentlayer (CallFunction|GetCurrentLayer))
          (if (== _layer0ref _currentlayer)
            (Variables|Default|SetNumberOfStairs (Variables|/Game/GameContent/Blueprints/interactives/MoveComponents/PassageBP.PassageBP_C|GetNumberOfStairs _aspassage_bp))
            (Variables|Default|SetStairsBPRef _aspassage_bp)
            (Pawn|Components|CharacterMovement|SetMovementMode (Variables|Character|GetCharacterMovement) "MOVE_Custom" 0)
            (Variables|Default|SetIsWalkingUp true)
            (goto _label Break)))))))

(event Input|EnhancedActionEvents|EnhancedInputActionIA_move_left
  (params (ActionValue :type Float%20%28double-precision%29) (ElapsedSeconds :type Float%20%28double-precision%29) (TriggeredSeconds :type Float%20%28double-precision%29) (InputAction :type Input%20Action%20Object%20Reference :default "/Game/GameContent/Blueprints/IA_move_left.IA_move_left"))
  (bind _returnvalue (Transformation|GetActorLocation))
  (bind _returnvalue_2 (Transformation|GetActorLocation))
  (bind _springarm (Variables|Default|GetSpringArm))
  (bind _returnvalue_3 (+ (.z _returnvalue_2) 4.0))
  ;[1 1 1] Controls
  (bind _candosth (CallFunction|CanDoSth))
  (if _candosth
    (Pawn|Input|AddMovementInput "1.000000,0.000000,0.000000" -1.0 false)
    (bind _layerwidth (CallFunction|GetCurrentLayer))
    (if (not (<= (.x _returnvalue) (- _layerwidth (* _layerwidth 2.0))))
      (if (not (>= (.x _returnvalue) _layerwidth))
        (Transformation|SetWorldLocation _springarm (Math|Vector|MakeVector (.x _returnvalue_2) 0.0 _returnvalue_3) false false)
        (else
          (Transformation|SetWorldLocation _springarm (Math|Vector|MakeVector _layerwidth 0.0 _returnvalue_3) false false)))
      (else
        (Transformation|SetWorldLocation _springarm (Math|Vector|MakeVector (- _layerwidth (* _layerwidth 2.0)) 0.0 _returnvalue_3) false false)))))

(event Input|EnhancedActionEvents|EnhancedInputActionIA_move_right
  (params (ActionValue :type Float%20%28double-precision%29) (ElapsedSeconds :type Float%20%28double-precision%29) (TriggeredSeconds :type Float%20%28double-precision%29) (InputAction :type Input%20Action%20Object%20Reference :default "/Game/GameContent/Blueprints/IA_move_right.IA_move_right"))
  (bind _returnvalue (Transformation|GetActorLocation))
  (bind _returnvalue_2 (Transformation|GetActorLocation))
  (bind _springarm (Variables|Default|GetSpringArm))
  (bind _returnvalue_3 (+ (.z _returnvalue) 4.0))
  ;[1 1 1] Controls
  (bind _candosth (CallFunction|CanDoSth))
  (if _candosth
    (Pawn|Input|AddMovementInput "1.000000,0.000000,0.000000" 1.0 false)
    (bind _layerwidth (CallFunction|GetCurrentLayer))
    (if (not (<= (.x _returnvalue_2) (- _layerwidth (* _layerwidth 2.0))))
      (if (not (>= (.x _returnvalue_2) _layerwidth))
        (Transformation|SetWorldLocation _springarm (Math|Vector|MakeVector (.x _returnvalue) 0.0 _returnvalue_3) false false)
        (else
          (Transformation|SetWorldLocation _springarm (Math|Vector|MakeVector _layerwidth 0.0 _returnvalue_3) false false)))
      (else
        (Transformation|SetWorldLocation _springarm (Math|Vector|MakeVector (- _layerwidth (* _layerwidth 2.0)) 0.0 _returnvalue_3) false false)))))

(event Input|EnhancedActionEvents|EnhancedInputActionIA_walk_down
  (params (ActionValue :type Float%20%28double-precision%29) (ElapsedSeconds :type Float%20%28double-precision%29) (TriggeredSeconds :type Float%20%28double-precision%29) (InputAction :type Input%20Action%20Object%20Reference :default "/Game/GameContent/Blueprints/IA_walk_down.IA_walk_down"))
  (bind _returnvalue (Transformation|GetActorLocation))
  ;[1 1 1] Controls
  (bind _candosth (CallFunction|CanDoSth))
  (if _candosth
    (bind _array_element (Utilities|Array|ForEachLoopwithBreak (Collision|GetOverlappingActors "/Game/GameContent/Blueprints/interactives/InteractiveBaseBP.InteractiveBaseBP_C" :!class /Script/Engine.Actor) :!label _label)
      (:LoopBody
        (if (Actor|ActorHasTag _array_element "MoveComponent")
          (bind _aspassage_bp (Utilities|Casting|CastToPassageBP _array_element))
          (bind _layer1ref (Default|GetLayers _aspassage_bp))
          (bind _currentlayer (CallFunction|GetCurrentLayer))
          (if (== _layer1ref _currentlayer)
            (Variables|Default|SetNumberOfStairs (Variables|/Game/GameContent/Blueprints/interactives/MoveComponents/PassageBP.PassageBP_C|GetNumberOfStairs _aspassage_bp))
            (Variables|Default|SetStairsBPRef _aspassage_bp)
            (Pawn|Components|CharacterMovement|SetMovementMode (Variables|Character|GetCharacterMovement) "MOVE_Custom" 0)
            (Transformation|Teleport (Math|Vector|MakeVector (.x _returnvalue) (+ (.y _returnvalue) 1.5e+02) (.z _returnvalue)) "0, 0, 0")
            (bind _asplayer_anim_bp (Utilities|Casting|CastToPlayerAnimBP (Variables|/Script/PaperZD.PaperZDAnimationComponent|GetAnimInstance (Variables|Default|GetPaperZDAnimation))))
            (Variables|Default|SetIsWalkingDown true)
            (Variables|/Game/GameContent/Blueprints/player/PlayerAnimBP.PlayerAnimBP_C|SetDown0 _asplayer_anim_bp true)
            (goto _label Break)))))))

(event Input|EnhancedActionEvents|EnhancedInputActionIA_interact
  (params (ActionValue :type Float%20%28double-precision%29) (ElapsedSeconds :type Float%20%28double-precision%29) (TriggeredSeconds :type Float%20%28double-precision%29) (InputAction :type Input%20Action%20Object%20Reference :default "/Game/GameContent/Blueprints/IA_interact.IA_interact"))
  (bind _dialogueui (Variables|Default|GetDialogueUI))
  ;[1 1 1] Controls
  (if (Variables|Default|GetIsSitting)
    (Variables|Default|SetIsGettingUp true)
    (else
      (bind _array_element (Utilities|Array|ForEachLoopwithBreak (Collision|GetOverlappingActors "/Game/GameContent/Blueprints/interactives/InteractiveBaseBP.InteractiveBaseBP_C" :!class /Script/Engine.Actor) :!label _label)
        (:LoopBody
          (bind _asnpc_bp (Utilities|Casting|CastToNpcBP _array_element)
            (:then
              (if (not (Variables|Default|GetIsUIOpened))
                (bind _candosth (CallFunction|CanDoSth))
                (if _candosth
                  (if (Utilities|DoesObjectImplementInterface _asnpc_bp "/Game/GameContent/Blueprints/interactives/npc/DialogueBP.DialogueBP_C")
                    (Variables|Default|SetIsUIOpened true)
                    (UserInterface|Viewport|AddtoViewport _dialogueui 0)
                    (Default|OpenUI _dialogueui self _asnpc_bp)
                    (goto _label Break)))
                (else
                  (Class|DialogueBP|Triggered(Message) _asnpc_bp)
                  (Default|Triggered (Variables|Default|GetDialogueUI)))))
            (:CastFailed
              (bind _candosth_2 (CallFunction|CanDoSth))
              (if _candosth_2
                (bind _asinteractive_object_bp (Utilities|Casting|CastToInteractiveObjectBP _array_element))
                (Variables|Default|SetInteractiveObjectRef _asinteractive_object_bp)
                (Default|OnInteract _asinteractive_object_bp self)
                (goto _label Break)))))))))

(event EventBeginPlay
  (bind _returnvalue (Transformation|GetActorLocation))
  (bind _returnvalue_2 (UserInterface|CreateWidget "/Game/GameContent/HUD.HUD_C"))
  (bind _output_get (Variables|Default|SetNewVar _returnvalue_2))
  (UserInterface|Viewport|AddtoViewport _output_get 0)
  (Input|SetInputModeGameOnly (Game|GetPlayerController 0) false)
  (bind _asplayer_controller (Utilities|Casting|CastToPlayerController (Pawn|GetController)))
  (Utilities|IsValid (PlayerController|LocalPlayerSubsystems|GetEnhancedInputLocalPlayerSubsystem _asplayer_controller)
    (:Is%20Valid
      (Input|AddMappingContext (PlayerController|LocalPlayerSubsystems|GetEnhancedInputLocalPlayerSubsystem _asplayer_controller) "/Game/GameContent/Blueprints/game_mapping_context.game_mapping_context" 0 "(bIgnoreAllPressedKeysUntilRelease=True,bForceImmediately=False,bNotifyUserSettings=False)")
      (bind _returnvalue_3 (UserInterface|CreateWidget "/Game/GameContent/InventoryUI.InventoryUI_C"))
      (Variables|Default|SetInventoryUI _returnvalue_3)
      (bind _returnvalue_4 (UserInterface|CreateWidget "/Game/GameContent/DialogueUI.DialogueUI_C"))
      (Variables|Default|SetDialogueUI _returnvalue_4)
      (Transformation|SetWorldLocation (Variables|Default|GetSpringArm) (Math|Vector|MakeVector (.x _returnvalue) (.y _returnvalue) (+ (.z _returnvalue) 4.0)) false false))))

(event EventTick
  (params (DeltaSeconds :type Float%20%28single-precision%29))
  (CallFunction|UpdateControlRotation)
  (CallFunction|IdleTimerEvent DeltaSeconds))

(fn ConstructionScript)

(fn Climb
  (bind _wall_height (Variables|Default|GetWall%20Height))
  (bind _sprite (Variables|Default|GetSprite))
  (bind (_x _y _z) (Math|Vector|BreakVector _wall_height))
  (Transformation|Teleport (Math|Vector|MakeVector (.X (Math|Vector|BreakVector (Variables|Default|GetWall%20Location))) _y (+ _z 2e+01)) "0, 0, 0")
  (Components|Timeline|SetLooping _sprite true)
  (Variables|Default|SetIsClimbing false)
  (Variables|Default|SetIsHanging false)
  (Pawn|Components|CharacterMovement|SetMovementMode (Variables|Character|GetCharacterMovement) "MOVE_Walking" 0)
  (Audio|Components|Audio|Play _sprite))

(fn CanDoSth
  (return (Math|Boolean|ANDBoolean (not (Variables|Default|GetIsWalkingUp)) (not (Variables|Default|GetIsWalkingDown)) (not (Variables|Default|GetIsUIOpened)) (not (Variables|Default|GetIsSittingDown)) (not (Variables|Default|GetIsSitting)) (not (Variables|Default|GetIsGettingUp)))))

(fn GetCurrentLayer
  (bind _currentlayer (Variables|Default|GetCurrentLayer))
  (Utilities|Casting|CastToLayerBP _currentlayer
    (:then
      (return _currentlayer (Variables|/Game/GameContent/Blueprints/level/LayerBP.LayerBP_C|GetLayerWidth _currentlayer)))
    (:CastFailed
      (return 0 3e+02))))